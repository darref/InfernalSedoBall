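; Player ball character that rolls automatically along the road spline, with sideways impulse steering and jumping.
; A looping timer adds movement along the closest spline direction, spins the mesh and turns the control rotation to follow the road.
; Damage reduces life; death respawns the ball near the spline start, refills life, restores red balls and restarts movement after a delay.
; Nearing the last spline point stops it and shows the end-of-level widget.
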(event `self.ReceiveTick`
  (params (DeltaSeconds :type "Float (single-precision)"))
  (bind _returnvalue (`GameplayStatics.GetActorOfClass` "/Game/PROJECT/ROAD/BP_RoadMotherClass.BP_RoadMotherClass_C"))
  (bind _spline (`/Game/PROJECT/ROAD/BP_Road_1.Spline` _returnvalue))
  (if (< (`KismetMathLibrary.Vector_Distance` (`SplineComponent.GetLocationAtSplinePoint` _spline (- (`SplineComponent.GetNumberOfSplinePoints` _spline) 1) "World") (`self.K2_GetActorLocation`)) 1500.0)
    (`/Engine/EditorBlueprintResources/StandardMacros.DoOnce` false
      (:`Completed`
        (`self.StopMoving`)
        (`self.EndOfLevel`)))))

(event `self.ReceiveAnyDamage`
  (params (Damage :type "Float (single-precision)") (DamageType :type "DamageType Object Reference") (InstigatedBy :type "Controller Object Reference") (DamageCauser :type "Actor Object Reference"))
  (bind _returnvalue (* (`KismetMathLibrary.Abs_Int` (`KismetMathLibrary.FTrunc` Damage)) -1))
  (`KismetSystemLibrary.PrintString` (`KismetStringLibrary.Conv_IntToString` _returnvalue))
  (bind _dead (`self.addRemoveLife` _returnvalue))
  (if _dead
    (`self.Dying`)))

(event `EndOfLevel`
  (bind _returnvalue (`|CreateWidget` "/Game/PROJECT/UI/W_endOfLevel.W_endOfLevel_C"))
  (`UserWidget.AddToViewport` _returnvalue 0)
  (set `PlayerController.bShowMouseCursor` true (`GameplayStatics.GetPlayerController` 0)))

(event `self.ReceiveBeginPlay`
  (`self.StartMoving`))

(event `StopMoving`
  (`KismetSystemLibrary.K2_PauseTimerHandle` (`self.MovingTimer`))
  (`MovementComponent.StopMovementImmediately` (`self.CharacterMovement`)))

(event `Moving`
  (bind _speed (`self.Speed`))
  (bind _returnvalue (`GameplayStatics.GetActorOfClass` "/Game/PROJECT/ROAD/BP_RoadMotherClass.BP_RoadMotherClass_C"))
  (bind _returnvalue_2 (`SplineHelper.getClosestDirectionOnSpline` (`/Game/PROJECT/ROAD/BP_Road_1.Spline` _returnvalue) (`self.K2_GetActorLocation`)))
  (`self.AddMovementInput` _returnvalue_2 _speed)
  (`SceneComponent.K2_AddLocalRotation` (`self.StaticMesh`) (`KismetMathLibrary.MakeRotator` 0.0 (* _speed -1.0 (`KismetSystemLibrary.K2_GetTimerElapsedTimeHandle` (`self.MovingTimer`)))) false false)
  (`Controller.SetControlRotation` (`GameplayStatics.GetPlayerController` 0) (`KismetMathLibrary.Conv_VectorToRotator` _returnvalue_2)))

(event `StartMoving`
  (bind _returnvalue (`KismetSystemLibrary.K2_SetTimer` null "Moving" 0.001 true))
  (set `self.MovingTimer` _returnvalue))

(event `Dying`
  (`self.StopMoving`)
  (bind _returnvalue (`GameplayStatics.GetActorOfClass` "/Game/PROJECT/ROAD/BP_RoadMotherClass.BP_RoadMotherClass_C"))
  (bind _spline (`/Game/PROJECT/ROAD/BP_Road_1.Spline` _returnvalue))
  (`self.K2_SetActorTransform` (`KismetMathLibrary.MakeTransform` (+ (`SplineComponent.GetLocationAtDistanceAlongSpline` _spline 1000.0 "World") (0.0 0.0 500.0)) (`KismetMathLibrary.Conv_VectorToRotator` (`SplineComponent.GetDirectionAtDistanceAlongSpline` _spline 1000.0 "World")) (0.5 0.5 0.5)))
  (set `self.life` (`self.lifeMax`))
  (`Controller.SetControlRotation` (`GameplayStatics.GetPlayerController` 0) (`KismetMathLibrary.Conv_VectorToRotator` (`SplineHelper.getClosestDirectionOnSpline` _spline (`self.K2_GetActorLocation`))))
  (bind _outactors (`GameplayStatics.GetAllActorsOfClass` "/Game/PROJECT/Traps/Redballs/BP_RedBalls.BP_RedBalls_C"))
  (for _array_element _outactors
    (`self.SetActorHiddenInGame` _array_element false)
    (`PrimitiveComponent.SetCollisionResponseToAllChannels` (`/Game/PROJECT/Traps/Redballs/BP_RedBalls.StaticMesh` _array_element) "ECR_Block")
    (`PrimitiveComponent.SetCollisionResponseToAllChannels` (`/Game/PROJECT/Traps/Redballs/BP_RedBalls.Sphere` _array_element) "ECR_Block"))
  (`KismetSystemLibrary.Delay` 2.0)
  (`self.StartMoving`))

(event `InputAxis|MoveRight`
  (params (AxisValue :type "Float (single-precision)"))
  (`CharacterMovementComponent.AddImpulse` (`self.CharacterMovement`) (* AxisValue (`self.Speed`) (`self.GetActorRightVector`)) true))

(event `InputAction|Jump`
  (params (Key :type "Key Structure"))
  (:`Pressed`
    (`self.Jump`)))

(fn `addRemoveLife`
  (params (Amount :type Integer))
  (returns (dead :type Boolean))
  (bind _returnvalue (+ (`self.life`) (`local.Amount`)))
  (bind _returnvalue_2 (+ (`self.life`) (`local.Amount`)))
  (if (< Amount 0)
    (if (<= _returnvalue_2 0)
      (set `self.life` 0)
      (return true)
      (else
        (set `self.life` _returnvalue_2)
        (return false)))
    (elif (>= _returnvalue (`self.lifeMax`))
      (set `self.life` (`self.lifeMax`))
      (return false)
      (else
        (set `self.life` _returnvalue)
        (return false)))))

(fn `UserConstructionScript`)