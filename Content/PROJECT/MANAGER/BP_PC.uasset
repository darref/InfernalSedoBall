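; BP_PC is a player controller that starts a level and gives the player a ball character on the road.
; StartGame streams in the named level, unloads the previous one tracked in BP_GameInstance, then replaces any existing ball.
; The new ball spawns above a point along the BP_RoadMotherClass spline, facing along it, and is possessed.
; BeginPlay starts Map_1 after a short delay, and left click shows the mouse cursor.
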(event `StartGame`
  (params (levelName :type Name))
  (`GameplayStatics.LoadStreamLevel` levelName true true)
  (bind _asbp_game_instance (cast `/Game/PROJECT/MANAGER/BP_GameInstance` (`GameplayStatics.GetGameInstance`)))
  (bind _output_get (set `self.tmpLevel` (`/Game/PROJECT/MANAGER/BP_GameInstance.currentLevel` _asbp_game_instance)))
  (`GameplayStatics.UnloadStreamLevel` _output_get true)
  (set `/Game/PROJECT/MANAGER/BP_GameInstance.currentLevel` levelName _asbp_game_instance)
  (bind _returnvalue (`GameplayStatics.GetActorOfClass` "/Game/PROJECT/ROAD/BP_RoadMotherClass.BP_RoadMotherClass_C"))
  (bind _charball (`self.charball`)
    (:`then`
      (`self.K2_DestroyActor` _charball))
    (:`else`
      _))
  (bind _spline (`/Game/PROJECT/ROAD/BP_Road_1.Spline` _returnvalue))
  (bind _returnvalue_2 (`|SpawnActorFromClass` "/Game/PROJECT/BallCharacter/BP_ballChar.BP_ballChar_C" (`KismetMathLibrary.MakeTransform` (+ (`SplineComponent.GetLocationAtDistanceAlongSpline` _spline 1000.0 "World") (0.0 0.0 500.0)) (`KismetMathLibrary.Conv_VectorToRotator` (`SplineComponent.GetDirectionAtDistanceAlongSpline` _spline 1000.0 "World"))) "Undefined" "OverrideRootScale" null null))
  (bind _output_get_2 (set `self.charball` _returnvalue_2))
  (`self.Possess` _output_get_2))

(event `self.ReceiveBeginPlay`
  (`KismetSystemLibrary.Delay` 3.0)
  (`self.StartGame` "Map_1"))

(event `Key|LeftMouseButton`
  (params (Key :type "Key Structure"))
  (:`Pressed`
    (set `self.bShowMouseCursor` true)))

(fn `UserConstructionScript`)