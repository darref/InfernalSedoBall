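; BP_RedBalls is a red ball pickup, filed under Traps, that affects the player's ball character when overlapped.
; On overlap with a BP_ballChar, it applies negative damage and enlarges the character's current scale by half.
; It then hides itself and sets its static mesh and sphere to ignore all collision channels, rather than destroying the actor.
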(event `self.ReceiveActorBeginOverlap`
  (params (OtherActor :type "Actor Object Reference"))
  (bind _asbp_ball_char (cast `/Game/PROJECT/BallCharacter/BP_ballChar` OtherActor))
  (`GameplayStatics.ApplyDamage` _asbp_ball_char -2.0 null self)
  (bind _returnvalue (`self.GetActorScale3D` _asbp_ball_char))
  (`self.SetActorScale3D` _asbp_ball_char (+ _returnvalue (* _returnvalue 0.5)))
  (`self.SetActorHiddenInGame` true)
  (`PrimitiveComponent.SetCollisionResponseToAllChannels` (`self.StaticMesh`) "ECR_Ignore")
  (`PrimitiveComponent.SetCollisionResponseToAllChannels` (`self.Sphere`) "ECR_Ignore"))

(fn `UserConstructionScript`)